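; BP_Pawn is a pawn Blueprint that turns MoveForward and TurnRight axis input into movement input, gated by a DisableMovement flag.
; Both events put control yaw into the rotator's roll with zero pitch and yaw, so the forward vector stays world +X.
; MoveForward scales by its amplified axis value, while TurnRight ignores its axis and applies constant forward input rather than turning.
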(event `InputAxis|MoveForward`
  (params (AxisValue :type "Float (single-precision)"))
  (if (not (`self.DisableMovement`))
    (`self.AddMovementInput` (`KismetMathLibrary.GetForwardVector` (`KismetMathLibrary.MakeRotator` (.yaw (`self.GetControlRotation`)))) (* AxisValue 5.0))))

(event `InputAxis|TurnRight`
  (params (AxisValue :type "Float (single-precision)"))
  (if (not (`self.DisableMovement`))
    (`self.AddMovementInput` (`KismetMathLibrary.GetForwardVector` (`KismetMathLibrary.MakeRotator` (.yaw (`self.GetControlRotation`)))))))

(fn `UserConstructionScript`)